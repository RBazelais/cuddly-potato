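; Turret actor that spots the third-person player through PawnSensing, turns to face them and fires projectiles with sound and explosion effects.
; Each sighting raises an in-range flag for roughly one sensing interval, letting Tick set yaw directly to the player, while RInterpTo affects only pitch and roll.
; A DoOnce with a one-second delayed reset paces forward-impulse shots.
; Foundation's world rotation is zeroed every tick, keeping the base still.
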(event OnSeePawn(PawnSensing)
  (params (Pawn :type Pawn%20Object%20Reference))
  ;[1 1 1] Can you see me now? How about now?
  (bind _asbp_third_person_character (Utilities|Casting|CastToBP_ThirdPersonCharacter Pawn))
  (Variables|Default|SetAs%20BP%20Third%20Person%20Character _asbp_third_person_character)
  (Variables|Default|SetIsPlayerInRange true)
  (Utilities|FlowControl|Delay (- (Variables|/Script/AIModule.PawnSensingComponent|GetSensingInterval (Variables|Default|GetPawnSensing)) (Class|Actor|GetActorTickInterval)))
  (Variables|Default|SetIsPlayerInRange false))

(event EventBeginPlay)

(event Collision|EventActorBeginOverlap
  (params (OtherActor :type Actor%20Object%20Reference)))

(event EventTick
  (params (DeltaSeconds :type Float%20%28single-precision%29))
  (bind _returnvalue (Transformation|GetActorRotation))
  (bind _returnvalue_2 (Utilities|Time|GetWorldDeltaSeconds))
  (bind _returnvalue_3 (Transformation|GetActorRotation))
  (bind _as_bp_third_person_character (Variables|Default|GetAs%20BP%20Third%20Person%20Character))
  (bind _projectilespawn2 (Variables|Default|GetProjectileSpawn2))
  (bind _returnvalue_4 (Math|Rotator|MakeRotator (.roll _returnvalue_3) (.pitch _returnvalue_3) (.yaw _returnvalue_3)))
  (bind _returnvalue_5 (Transformation|GetWorldLocation _projectilespawn2))
  (bind _returnvalue_6 (Math|Interpolation|RInterpTo _returnvalue _returnvalue_4 _returnvalue_2 5.0))
  (Transformation|SetWorldRotation (Variables|Default|GetFoundation) "0, 0, 0" false false)
  (Utilities|IsValid _as_bp_third_person_character
    (:Is%20Valid
      (if (Variables|Default|GetIsPlayerInRange)
        (Transformation|SetActorRotation (Math|Rotator|MakeRotator (.roll _returnvalue_6) (.pitch _returnvalue_6) (.yaw (Math|Rotator|FindLookatRotation (Transformation|GetActorLocation) (Transformation|GetActorLocation _as_bp_third_person_character)))))
        ;[1 1 1] Wait 1 sec to reset
        (Utilities|FlowControl|DoOnce false :!label _label
          (:Completed
            (Utilities|FlowControl|Sequence
              (:then_0
                (Audio|PlaySoundatLocation "/Game/StarterContent/Audio/Explosion_Cue.Explosion_Cue" (Transformation|GetActorLocation) "0, 0, 0" 1.0 1.0 0.0 0 0 0 0)
                (Game|SpawnActorfromClass "/Game/Turret/BP_Projectile2.BP_Projectile2_C" (Math|Transform|MakeTransform _returnvalue_5 "0, 0, 0" "1.000000,1.000000,1.000000") "Undefined" 0 (* (Transformation|GetActorForwardVector) (Variables|Default|GetFireStrength)) 0)
                (Effects|SpawnEmitteratLocation "/Game/StarterContent/Particles/P_Explosion.P_Explosion" _returnvalue_5 "0, 0, 0" "0.250000,0.250000,0.250000"))
              (:then_1
                (Utilities|FlowControl|Delay 1.0)
                (goto _label Reset)))))))))

(fn ConstructionScript
  (Transformation|SetWorldRotation (Variables|Default|GetFoundation) "0, 0, 0" false false))